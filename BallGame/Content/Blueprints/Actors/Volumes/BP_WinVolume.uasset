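; BP_WinVolume is a volume actor that acts as the level's win trigger, gated on collecting every coin.
; When the player overlaps it, AnyActorsOnLevel searches for BP_collectable actors and, despite its name, returns true when none remain.
; That result calls CompleteLevel, otherwise a Polish "not all coins collected" message is printed.
; CompleteLevel is unfinished: it only gets the current level name, and LevelNames is unused.
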(event EventBeginPlay)

(event EventTick
  (params (DeltaSeconds :type Float%20%28single-precision%29)))

(event Collision|EventActorBeginOverlap
  (params (OtherActor :type Actor%20Object%20Reference))
  (Utilities|IsPlayer OtherActor
    (:IsPlayer
      (if (CallFunction|AnyActorsonLevel)
        (CallFunction|CompleteLevel)
        (else
          (Development|PrintString "Nie zebrales wszystkich monet"))))))

(fn ConstructionScript)

(fn AnyActorsonLevel
  (bind _outactors (Actor|GetAllActorsOfClass "/Game/Blueprints/Actors/Collectables/BP_collectable.BP_collectable_C"))
  (return (>= 0 (Utilities|Array|Length _outactors))))

(fn CompleteLevel
  (Game|GetCurrentLevelName true))