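; BP_collectable is a pickup actor that plays a vanishing effect when the player pawn overlaps it.
; On overlap it caches its location, scale and point light intensity as lerp start values.
; The SmoothLerp timeline then moves it to a fixed world height, shrinks it to zero and fades the light, destroying the actor when finished.
; It awards nothing to the player itself.
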(event EventTick
  (params (DeltaSeconds :type Float%20%28single-precision%29)))

(event Collision|EventActorBeginOverlap
  (params (OtherActor :type Actor%20Object%20Reference))
  (if (== OtherActor (Game|Player|GetPlayerPawn 0))
    (CallFunction|SetActualValues)
    (bind (_direction _location _scale _intensity) (Timeline|SmoothLerp Play)
      (:Update
        (CallFunction|SetActorLocation _location)
        (CallFunction|SetActorScale _scale)
        (CallFunction|SetLightIntensity _intensity))
      (:Finished
        (Actor|DestroyActor)))))

(fn ConstructionScript)

(fn SetActualValues
  (Variables|Default|SetCollectableActualLocation (Transformation|GetActorLocation))
  (Variables|Default|SetCollectableActualScale (Transformation|GetActorScale3D))
  (Variables|Default|SetCollectableActualIntensity (Variables|/Script/Engine.LightComponentBase|GetIntensity (Variables|Default|GetPointLight))))

(fn SetActorLocation
  (params (Alpha :type Float%20%28single-precision%29))
  (bind _returnvalue (Transformation|GetActorLocation))
  (Transformation|SetActorLocation (Math|Vector|Lerp(Vector) (Variables|Default|GetCollectableActualLocation) (Math|Vector|MakeVector (.x _returnvalue) (.y _returnvalue) 2.4e+02) Alpha) false false))

(fn SetActorScale
  (params (Alpha :type Float%20%28single-precision%29))
  (Transformation|SetActorScale3D (Math|Vector|Lerp(Vector) (Variables|Default|GetCollectableActualScale) "0.0,0.0,0.000000" Alpha)))

(fn SetLightIntensity
  (params (Alpha :type Float%20%28single-precision%29))
  (Rendering|Components|Light|SetIntensity (Variables|Default|GetPointLight) (Math|Float|Lerp (Variables|Default|GetCollectableActualIntensity) 0.0 Alpha)))