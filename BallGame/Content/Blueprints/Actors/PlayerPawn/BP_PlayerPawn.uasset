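; Player pawn that rolls a sphere by physics torque and restarts the level when it takes damage.
; Left/right and forward/backward axis inputs share one torque call on the sphere, scaled by TorqueMultiplier and applied as an acceleration change.
; Any damage prints a debug message and runs ResetLevel, which fades the camera to black, waits, reopens the current level by name, then requests a fade back in.
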(event Game|Damage|EventAnyDamage
  (params (Damage :type Float%20%28single-precision%29) (DamageType :type Damage%20Type%20Object%20Reference) (InstigatedBy :type Controller%20Object%20Reference) (DamageCauser :type Actor%20Object%20Reference))
  (Development|PrintString "otrzymales obrazenia!" true true "(R=1.000000,G=0.000000,B=0.087764,A=1.000000)")
  (|ResetLevel))

(event Input|AxisEvents|InputAxisMoveforward/backwards
  (params (AxisValue :type Float%20%28single-precision%29))
  (Class|PrimitiveComponent|AddTorqueinRadians (Variables|Default|GetSphere) (Math|Vector|MakeVector (* (Variables|Default|GetTorque_multiplier) (stale Input|AxisEvents|InputAxisMoveleft/right AxisValue)) (* AxisValue (Variables|Default|GetTorque_multiplier)) 0.0) "None" true))

(event Input|AxisEvents|InputAxisMoveleft/right
  (params (AxisValue :type Float%20%28single-precision%29))
  (Class|PrimitiveComponent|AddTorqueinRadians (Variables|Default|GetSphere) (Math|Vector|MakeVector (* (Variables|Default|GetTorque_multiplier) AxisValue) (* (stale Input|AxisEvents|InputAxisMoveforward/backwards AxisValue) (Variables|Default|GetTorque_multiplier)) 0.0) "None" true))

(fn ConstructionScript)